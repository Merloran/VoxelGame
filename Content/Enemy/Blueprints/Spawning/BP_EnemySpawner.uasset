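; Enemy spawner that, between StartSpawning and StopSpawning calls, periodically asks the enemy subsystem to spawn enemies of one type within a position range.
; A looping timer with an adjusted initial delay fires Spawn, sampling a progression curve at an elapsed counter to set each wave's size.
; The counter advances by the interval, but holds or optionally resets past its maximum while BP_EnemyManager is below its enemy cap.
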(event `Spawn`
  (`EnemySubsystem.SpawnEnemies` (subsystem `EnemySubsystem`) (`self.SpawnedType`) (`KismetMathLibrary.FTrunc` (`CurveFloat.GetFloatValue` (`self.CurveProgression`) (`self.InnerCounter`))) (`self.EnemyData`) (`self.MinSpawnPosition`) (`self.MaxSpawnPosition`))
  (bind _returnvalue (`GameplayStatics.GetActorOfClass` "/Game/Enemy/BP_EnemyManager.BP_EnemyManager_C"))
  (if (and (< (`KismetArrayLibrary.Array_Length` (`/Game/Enemy/BP_EnemyManager.Enemies` _returnvalue)) (`/Game/Enemy/BP_EnemyManager.MaxEnemiesCount` _returnvalue)) (>= (`self.InnerCounter`) (`self.MaxProgression`)))
    (if (`self.ResetProgression`)
      (set `self.InnerCounter` 0.0))
    (else
      (set `self.InnerCounter` (+ (`self.InnerCounter`) (`self.SpawnInterval`))))))

(event `BeginSpawning`
  (bind _spawninterval (`self.SpawnInterval`))
  (bind _returnvalue (`KismetSystemLibrary.K2_SetTimerDelegate` (delegate `Spawn`) _spawninterval true false (- (`self.SpawnDelay`) _spawninterval)))
  (set `self.TimerHandle` _returnvalue))

(event `self.ReceiveBeginPlay`)

(fn `StartSpawning`
  (`self.BeginSpawning`))

(fn `StopSpawning`
  (bind _timerhandle (`self.TimerHandle`))
  (if (`KismetSystemLibrary.K2_IsValidTimerHandle` _timerhandle)
    (`KismetSystemLibrary.K2_ClearAndInvalidateTimerHandle` _timerhandle)))

(fn `UserConstructionScript`)