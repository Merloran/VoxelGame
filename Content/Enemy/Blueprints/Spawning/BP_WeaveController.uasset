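; BP_WeaveController runs the enemy wave cycle, starting a wave on play and creating a next-wave button widget linked to itself.
; Each wave selects its spawner set and duration, with the third set as fallback, then starts spawning and switches DayLight off.
; When the timer ends, it stops spawners, clears enemies through EnemyManager, restores the light, shows the button and has the player character spawn a tram.
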(event `self.ReceiveBeginPlay`
  (bind _returnvalue (`|CreateWidget` "/Game/UI/WBP_Button_NextWave.WBP_Button_NextWave_C"))
  (bind _output_get (set `self.NextWaveButton` _returnvalue))
  (`/Game/UI/WBP_Button_NextWave.SetWeaveController` _output_get self)
  (`UserWidget.AddToViewport` (`self.NextWaveButton`) 0)
  (`self.StartNextWeave`))

(event `FinishWeave`
  (for _array_element (`self.CurrentSpawners`)
    (`/Game/Enemy/Blueprints/Spawning/BP_EnemySpawner.StopSpawning` _array_element))
  (`/Game/Enemy/BP_EnemyManager.ClearEnemies` (`self.EnemyManager`))
  (`Widget.SetVisibility` (`self.NextWaveButton`) "Visible")
  (set `self.WeaveIsActive` false)
  (`LightComponent.SetIntensity` (`Light.LightComponent` (`self.DayLight`)) 2.0)
  (bind _asbp_third_person_character (cast `/Game/ThirdPerson/Blueprints/BP_ThirdPersonCharacter` (`GameplayStatics.GetPlayerPawn` 0)))
  (`/Game/ThirdPerson/Blueprints/BP_ThirdPersonCharacter.SpawnTram` _asbp_third_person_character))

(event `BeginWeave`
  (for _array_element (`self.CurrentSpawners`)
    (`/Game/Enemy/Blueprints/Spawning/BP_EnemySpawner.StartSpawning` _array_element))
  (`KismetSystemLibrary.K2_SetTimerDelegate` (delegate `FinishWeave`) (`self.CurrentWeaveTime`))
  (`LightComponent.SetIntensity` (`Light.LightComponent` (`self.DayLight`)) 0.0))

(fn `StartNextWeave`
  (if (not (`self.WeaveIsActive`))
    (bind _result (`/Engine/EditorBlueprintResources/StandardMacros.IncrementInt` (`self.WeaveNumber`))
      (:`  `
        (`self.StartWeave` _result)))))

(fn `StartWeave`
  (params (WeaveNumber :type Integer))
  (`Widget.SetVisibility` (`self.NextWaveButton`) "Hidden")
  (set `self.WeaveIsActive` true)
  (switch `int` WeaveNumber
    (:`Default`
      (set `self.CurrentSpawners` (`self.W03_Spawners`) :!label _label)
      (set `self.CurrentWeaveTime` (`self.W03_Time`)))
    (:`1`
      (set `self.CurrentSpawners` (`self.W01_Spawners`))
      (set `self.CurrentWeaveTime` (`self.W01_Time`)))
    (:`2`
      (set `self.CurrentSpawners` (`self.W02_Spawners`))
      (set `self.CurrentWeaveTime` (`self.W02_Time`)))
    (:`3`
      (goto _label)))
  (`self.BeginWeave`))

(fn `UserConstructionScript`)