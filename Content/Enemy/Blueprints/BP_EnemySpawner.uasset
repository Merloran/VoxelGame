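; BP_EnemySpawner periodically spawns enemies of a configured type during play.
; BeginPlay starts a looping timer with a configurable interval and initial delay that fires the Spawn event.
; Spawn delegates to the EnemySubsystem, passing the enemy type, count, data and min/max position range, so the spawner itself only handles timing and configuration.
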(event `Spawn`
  (`EnemySubsystem.SpawnEnemies` (subsystem `EnemySubsystem`) (`self.SpawnedType`) (`self.SpawnedNumber`) (`self.EnemyData`) (`self.MinSpawnPosition`) (`self.MaxSpawnPosition`)))

(event `self.ReceiveBeginPlay`
  (`KismetSystemLibrary.K2_SetTimerDelegate` (delegate `Spawn`) (`self.SpawnInterval`) true false (`self.SpawnDelay`)))

(fn `UserConstructionScript`)