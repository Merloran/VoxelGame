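; BP_EnemyManager configures the EnemySubsystem for the game's enemies and offers functions to read or clear them.
; On BeginPlay it sets the MI_Swelling death material and registers Blueprint templates for the Rat and RatElite enemy types.
; GetAllEnemies returns its Enemies array, which nothing here populates.
; ClearEnemies destroys the valid actors in that array, empties it and calls ClearAll on the subsystem.
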(event `self.ReceiveBeginPlay`
  (bind _returnvalue (subsystem `EnemySubsystem`))
  (set `EnemySubsystem.EnemyDeathMaterial` "/Game/Materials/MI_Swelling.MI_Swelling" _returnvalue)
  (`EnemySubsystem.RegisterEnemyActorTemplate` _returnvalue "Rat" "/Game/Enemy/BP_Enemy.BP_Enemy_C")
  (`EnemySubsystem.RegisterEnemyActorTemplate` _returnvalue "RatElite" "/Game/Enemy/BP_Enemy_Elite.BP_Enemy_Elite_C"))

(fn `ClearEnemies`
  (bind _enemies (`self.Enemies`))
  (for _array_element _enemies
    (if (`KismetSystemLibrary.IsValid` _array_element)
      (`self.K2_DestroyActor` _array_element)))
  (`KismetArrayLibrary.Array_Clear` _enemies)
  (`EnemySubsystem.ClearAll` (subsystem `EnemySubsystem`)))

(fn `GetAllEnemies`
  (returns (enemies :type "Array of /Game/Enemy/BP_Enemy Object Reference"))
  (return (`self.Enemies`)))

(fn `UserConstructionScript`)