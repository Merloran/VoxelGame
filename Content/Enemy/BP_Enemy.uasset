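; BP_Enemy is an enemy actor that registers with the level's BP_EnemyManager and drops experience when destroyed.
; On BeginPlay it adds itself to the manager's Enemies array if not already there.
; When destroyed it removes itself and spawns an enlarged BP_ExpOrb slightly above its location.
; TakeDamage forwards damage to the EnemySubsystem, leaving older local health logic disconnected.
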(event `self.ReceiveBeginPlay`
  (bind _returnvalue (`GameplayStatics.GetActorOfClass` "/Game/Enemy/BP_EnemyManager.BP_EnemyManager_C"))
  (bind _enemies (`/Game/Enemy/BP_EnemyManager.Enemies` _returnvalue))
  (if (not (`KismetArrayLibrary.Array_Contains` _enemies self))
    (`KismetArrayLibrary.Array_Add` _enemies self)))

(event `self.ReceiveTick`
  (params (DeltaSeconds :type "Float (single-precision)")))

(event `self.ReceiveDestroyed`
  (bind _returnvalue (`GameplayStatics.GetActorOfClass` "/Game/Enemy/BP_EnemyManager.BP_EnemyManager_C"))
  (`KismetArrayLibrary.Array_RemoveItem` (`/Game/Enemy/BP_EnemyManager.Enemies` _returnvalue) self)
  (`|SpawnActorFromClass` "/Game/ThirdPerson/Blueprints/BP_ExpOrb.BP_ExpOrb_C" (`KismetMathLibrary.MakeTransform` (+ (`self.K2_GetActorLocation`) (0.0 0.0 100.0)) (struct) (2.0 2.0 2.0)) "Undefined" "MultiplyWithRoot" null null))

(fn `TakeDamage`
  (params (damage :type "Float (double-precision)") (attackType :type "/Game/ThirdPerson/Blueprints/weapons/E_AttackType Enum" :default "NewEnumerator0") (attackEffect :type "/Game/ThirdPerson/Blueprints/weapons/E_AttackEffect Enum" :default "NewEnumerator0"))
  (`EnemySubsystem.DamageEnemy` (subsystem `EnemySubsystem`) (`self.Enemy`) damage))

(fn `UserConstructionScript`)